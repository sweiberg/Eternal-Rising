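; Test instancer actor for AnimToTexture that gives each static mesh instance a randomized auto-play animation from a data asset.
; After the parent construction script runs, it builds one auto-play entry per instance with a random animation index and time offset.
; The entries are batch-applied to the instanced mesh along with the instance transforms, all at construction time, leaving the event graph empty.
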(event EventBeginPlay)

(event Collision|EventActorBeginOverlap
  (params (OtherActor :type Actor%20Object%20Reference)))

(event EventTick
  (params (DeltaSeconds :type Float%20%28single-precision%29)))

(fn ConstructionScript
  (Variables|Default|SetAuto%20Play true)
  (|CallParentFunction)
  (bind _autoplaydata (CallFunction|BuildAutoPlayData (Variables|Default|GetInstancedStaticMesh) (Variables|Default|GetDataAsset)))
  (Class|AnimtoTextureInstancePlaybackLibrary|BatchUpdateInstancesAutoPlayData (Variables|Default|GetInstancedStaticMesh) _autoplaydata (Variables|Default|GetMatrices) true))

(fn BuildAutoPlayData
  (params (InstancedStaticMesh :type Instanced%20Static%20Mesh%20Component%20Object%20Reference) (DataAsset :type Anim%20to%20Texture%20Data%20Asset%20Object%20Reference))
  (Utilities|Array|Clear (LocalVariables|Get_AutoPlayData))
  (for _index (range 0 (- (Components|InstancedStaticMesh|GetInstanceCount InstancedStaticMesh) 1))
    (bind _autoplaydata (Class|AnimtoTextureInstancePlaybackLibrary|GetAutoPlayDatafromDataAsset DataAsset (Math|Random|RandomInteger (Utilities|Array|Length (Variables|/Script/AnimToTexture.AnimToTextureDataAsset|GetAnimations DataAsset))) (Math|Random|RandomFloatinRange 0.0 2e+01) 1.0))
    (Utilities|Array|Add (LocalVariables|Get_AutoPlayData) _autoplaydata))
  (return (LocalVariables|Get_AutoPlayData)))