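; BP_AmmunitionItem is an ammunition item actor that can reappear in the world after being hidden.
; Its construction script takes the static mesh from the Item data and enables physics simulation.
; RespawnTimer schedules RespawnAmmo after a fixed delay.
; RespawnAmmo unhides the item through the RPCShowActorServer call on player 0's BP_FirstPersonCharacter, rather than setting visibility itself.
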(event Custom|RespawnTimer
  (Utilities|Time|SetTimerbyFunctionName 0 "RespawnAmmo" 45.0))

(event Custom|RespawnAmmo
  (bind _asbp_first_person_character (Utilities|Casting|CastToBP_FirstPersonCharacter (Game|GetPlayerCharacter 0)))
  (Default|RPCShowActorServer _asbp_first_person_character self false))

(fn ConstructionScript
  (bind _staticmesh (Variables|Default|GetStaticMesh))
  (Components|StaticMesh|SetStaticMesh _staticmesh (.Mesh (Utilities|Struct|BreakItemStructure (Variables|Default|GetItem))))
  (Physics|SetSimulatePhysics _staticmesh true))