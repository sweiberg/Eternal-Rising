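; Player inventory component that holds a 15-slot item array, shows it in a SurvivorInventory widget and handles pickup.
; The inventory input toggles the widget, mouse cursor and input mode.
; Interact sphere-traces around the player's lower body for a BP_InventoryItem, then loops through slots to stack it under a quantity cap or fill empty ones.
; Pickups refresh the widget and destroy the world item locally and through the character's server RPC.
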(event Input|EnhancedActionEvents|EnhancedInputActionIA_SurvivorInventory
  (params (ActionValue :type Boolean) (ElapsedSeconds :type Float%20%28double-precision%29) (TriggeredSeconds :type Float%20%28double-precision%29) (InputAction :type Input%20Action%20Object%20Reference :default "/Game/Input/Actions/IA_SurvivorInventory.IA_SurvivorInventory"))
  (bind _returnvalue (Game|GetPlayerController 0))
  (bind _returnvalue_2 (Game|GetPlayerController 0))
  (bind _inventorywidget (Variables|Default|GetInventoryWidget))
  ;[1 1 1] Show / Hide Inventory
  (:Completed
    (if (Widget|IsVisible (Variables|Default|GetInventoryWidget))
      (Widget|RemovefromParent _inventorywidget)
      (Variables|/Script/Engine.PlayerController|SetbShowMouseCursor _returnvalue false)
      (Input|SetInputModeGameOnly _returnvalue false)
      (else
        (Variables|/Script/Engine.PlayerController|SetbShowMouseCursor _returnvalue_2 true)
        (Input|SetInputModeGameandUI _returnvalue_2 0 "DoNotLock" true false)
        (UserInterface|Viewport|AddtoViewport _inventorywidget 0)))))

(event Input|EnhancedActionEvents|EnhancedInputActionIA_SurvivorInteract
  (params (ActionValue :type Boolean) (ElapsedSeconds :type Float%20%28double-precision%29) (TriggeredSeconds :type Float%20%28double-precision%29) (InputAction :type Input%20Action%20Object%20Reference :default "/Game/Input/Actions/IA_SurvivorInteract.IA_SurvivorInteract"))
  (bind _returnvalue (Game|GetPlayerCharacter 0))
  (bind _returnvalue_2 (Transformation|GetActorLocation _returnvalue))
  (bind _returnvalue_3 (- _returnvalue_2 "0.000000,0.000000,65.000000"))
  ;[1 1 1] Pickup Item
  (:Completed
    (bind _outhit (Collision|SphereTraceByChannel _returnvalue_3 _returnvalue_3 1.2e+02 "TraceTypeQuery1" false 0 "None"))
    (bind _asbp_inventory_item (Utilities|Casting|CastToBP_InventoryItem (.HitActor (Collision|BreakHitResult _outhit))))
    (Utilities|IsValid _asbp_inventory_item
      (:Is%20Valid
        (for (_array_element _array_index) (Variables|Default|GetItems)
          (if (Math|Boolean|ANDBoolean (Utilities|Enum|Equal(Enum) (.Name (Utilities|Struct|BreakItemStructure _array_element)) (.Name (Utilities|Struct|BreakItemStructure (Variables|/Game/Blueprints/Player/BP_InventoryItem.BP_InventoryItem_C|GetItem _asbp_inventory_item)))) (.Stackable (Utilities|Struct|BreakItemStructure (Variables|/Game/Blueprints/Player/BP_InventoryItem.BP_InventoryItem_C|GetItem _asbp_inventory_item))) (<= (+ (.Quantity (Utilities|Struct|BreakItemStructure _array_element)) (.Quantity (Utilities|Struct|BreakItemStructure (Variables|/Game/Blueprints/Player/BP_InventoryItem.BP_InventoryItem_C|GetItem _asbp_inventory_item)))) 15))
            (Utilities|Array|SetArrayElem (Variables|Default|GetItems) _array_index (Utilities|Struct|MakeItemStructure (.name (Variables|/Game/Blueprints/Player/BP_InventoryItem.BP_InventoryItem_C|GetItem _asbp_inventory_item)) (.stackable (Variables|/Game/Blueprints/Player/BP_InventoryItem.BP_InventoryItem_C|GetItem _asbp_inventory_item)) (+ (.Quantity (Utilities|Struct|BreakItemStructure _array_element)) (.Quantity (Utilities|Struct|BreakItemStructure (Variables|/Game/Blueprints/Player/BP_InventoryItem.BP_InventoryItem_C|GetItem _asbp_inventory_item)))) (.thumbnail (Variables|/Game/Blueprints/Player/BP_InventoryItem.BP_InventoryItem_C|GetItem _asbp_inventory_item)) (.mesh (Variables|/Game/Blueprints/Player/BP_InventoryItem.BP_InventoryItem_C|GetItem _asbp_inventory_item))))
            (Default|LoadInventory (Variables|Default|GetInventoryWidget) self :!label _label)
            (bind _asbp_first_person_character (Utilities|Casting|CastToBP_FirstPersonCharacter (Game|GetPlayerCharacter 0)))
            (Default|RPCDestroyActorServer _asbp_first_person_character _asbp_inventory_item)
            (Actor|DestroyActor _asbp_inventory_item)
            (elif (== (.Quantity (Utilities|Struct|BreakItemStructure _array_element)) 0)
              (Utilities|Array|SetArrayElem (Variables|Default|GetItems) _array_index (Variables|/Game/Blueprints/Player/BP_InventoryItem.BP_InventoryItem_C|GetItem _asbp_inventory_item))
              (goto _label))))))))

(event EventBeginPlay
  ;[1 1 1] Load Inventory
  (bind _returnvalue (UserInterface|CreateWidget "/Game/Blueprints/UI/SurvivorInventory.SurvivorInventory_C"))
  (Variables|Default|SetInventoryWidget _returnvalue)
  (Utilities|Array|Resize (Variables|Default|GetItems) 15)
  (Default|LoadInventory (Variables|Default|GetInventoryWidget) self))