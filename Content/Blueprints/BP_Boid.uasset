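; BP_Boid is a boid actor that reacts to first-person projectile hits by fading its appearance and destroying itself.
; A hit on its instanced static mesh from BP_FirstPersonProjectile calls AppearanceMulti, then passes the projectile to ServerHandleHit, which is not defined in this graph.
; AppearanceMulti plays a timeline that drives the mesh materials' Appearance parameter and destroys the actor when finished.
; The graph contains no flocking logic.
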(event Custom|AppearanceMulti
  (bind _appearancevalue (Timeline|AppearanceTimeline Play)
    (:Update
      (Rendering|Material|SetScalarParameterValueonMaterials (Variables|Default|GetInstancedStaticMeshComponent) "Appearance" _appearancevalue))
    (:Finished
      (Actor|DestroyActor))))

(event EventBeginPlay)

(event Collision|EventActorBeginOverlap
  (params (OtherActor :type Actor%20Object%20Reference)))

(event EventTick
  (params (DeltaSeconds :type Float%20%28single-precision%29)))

(event Collision|EventHit
  (params (MyComp :type Primitive%20Component%20Object%20Reference) (Other :type Actor%20Object%20Reference) (OtherComp :type Primitive%20Component%20Object%20Reference) (bSelfMoved :type Boolean) (HitLocation :type Vector :default "0, 0, 0") (HitNormal :type Vector :default "0, 0, 0") (NormalImpulse :type Vector :default "0, 0, 0") (Hit :type Hit%20Result%20Structure%20%28by%20ref%29))
  (if (Class|GameplayStatics|ObjectIsA MyComp "/Script/Engine.InstancedStaticMeshComponent")
    (if (Class|GameplayStatics|ObjectIsA Other "/Game/FirstPerson/Blueprints/BP_FirstPersonProjectile.BP_FirstPersonProjectile_C")
      (bind _asbp_first_person_projectile (Utilities|Casting|CastToBP_FirstPersonProjectile Other))
      (Utilities|FlowControl|Sequence
        (:then_0
          (CallFunction|AppearanceMulti))
        (:then_1
          (Class|FlecsZombieBoid|ServerHandleHit _asbp_first_person_projectile))))))

(fn ConstructionScript)