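; Game mode for a two-player asymmetric match between a Director and a Survivor.
; Once two players are queued, the first gets a team-select HUD while the second spectates, and that choice assigns both roles.
; Round start spawns and possesses each role's pawn, sets HUDs, plays the Survivor intro, and starts round timers and the objective pad.
; It also updates role state on logout and handles map reload through server travel.
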(event Custom|AssignPlayersToRoles
  ;[0.01938 0.01938 0.01938] Player Assign
  (bind _asbp_survivor_controller_merge_test (Utilities|Casting|CastToBP_SurvivorControllerMergeTest (Utilities|Array|Get(acopy) (Variables|Default|GetPlayerQueue))))
  (Default|SetTeamSelectHUD _asbp_survivor_controller_merge_test)
  (bind _returnvalue (Actor|GetActorOfClass "/Game/Blueprints/Player/BP_DirectorStart.BP_DirectorStart_C"))
  (bind _returnvalue_2 (Game|SpawnActorfromClass "/Script/Engine.SpectatorPawn" (Transformation|GetActorTransform _returnvalue) "Undefined" "MultiplyWithRoot" 0 0))
  (Pawn|Possess (Utilities|Array|Get(acopy) (Variables|Default|GetPlayerQueue) 1) _returnvalue_2))

(event Custom|RoundStart
  (bind _directorplayer (Variables|Default|GetDirectorPlayer))
  (bind _survivorplayer (Variables|Default|GetSurvivorPlayer))
  ;[0.0356 0.0356 0.0356] Round Start
  (Utilities|FlowControl|Sequence
    (:then_0
      (bind _returnvalue (Actor|GetActorOfClass "/Game/Blueprints/Player/BP_DirectorStart.BP_DirectorStart_C"))
      (bind _returnvalue_2 (Game|SpawnActorfromClass "/Game/Blueprints/Player/DirectorPawnTest.DirectorPawnTest_C" (Transformation|GetActorTransform _returnvalue) "Undefined" "MultiplyWithRoot" 0 0))
      (Pawn|Possess _directorplayer _returnvalue_2)
      (Input|SetInputModeGameandUI _directorplayer 0 "LockAlways" true false)
      (Variables|/Script/Engine.PlayerController|SetbShowMouseCursor _directorplayer true)
      (Class|PlayerController|ClientSetHUD _directorplayer "/Game/Misc/BP_DirectorHUD.BP_DirectorHUD_C"))
    (:then_1
      (bind _returnvalue_3 (Actor|GetActorOfClass "/Game/Blueprints/Player/BP_SurvivorStart.BP_SurvivorStart_C"))
      (bind _returnvalue_4 (Game|SpawnActorfromClass "/Game/Blueprints/Player/BP_FirstPersonCharacter.BP_FirstPersonCharacter_C" (Transformation|GetActorTransform _returnvalue_3) "Undefined" "MultiplyWithRoot" 0 0))
      (Pawn|Possess _survivorplayer _returnvalue_4)
      (Class|PlayerController|ClientSetHUD _survivorplayer "/Game/Misc/BP_SurvivorHUD.BP_SurvivorHUD_C"))
    (:then_2
      (bind _asbp_survivor_controller_merge_test (Utilities|Casting|CastToBP_SurvivorControllerMergeTest (Variables|Default|GetSurvivorPlayer)))
      (Default|RPCPlaySoundClient _asbp_survivor_controller_merge_test "/Game/Sounds/Survivor_Introduction.Survivor_Introduction"))
    (:then_3
      (bind _outactors (Actor|GetAllActorsOfClass "/Game/Blueprints/UI/RoundTimer.RoundTimer_C"))
      (for _array_element _outactors
        (Default|StartRoundTimer _array_element))
      (bind _returnvalue_5 (Actor|GetActorOfClass "/Game/Blueprints/Object/ObjectivePad.ObjectivePad_C"))
      (Default|ObjectiveRoundStart _returnvalue_5))))

(event Custom|RPC_ReloadMapServer
  (Class|ServerGameMode|DoServerTravel))

(event Custom|RPC_UserTeamSelection
  (params (TeamNumber :type Integer))
  (bind _playerqueue (Variables|Default|GetPlayerQueue))
  (bind _playerqueue_2 (Variables|Default|GetPlayerQueue))
  ;[0.01938 0.01938 0.01938] Player Assign
  (if (== TeamNumber 1)
    (Variables|Default|SetDirectorPlayer (Utilities|Array|Get(acopy) _playerqueue 1))
    (Variables|Default|SetSurvivorPlayer (Utilities|Array|Get(acopy) _playerqueue))
    (CallFunction|RoundStart)
    (else
      (Variables|Default|SetDirectorPlayer (Utilities|Array|Get(acopy) _playerqueue_2))
      (Variables|Default|SetSurvivorPlayer (Utilities|Array|Get(acopy) _playerqueue_2 1))
      (CallFunction|RoundStart))))

(event EventOnLogout
  (params (ExitingController :type Controller%20Object%20Reference))
  ;[0.01938 0.01938 0.01938] Player Disconnect
  (if (== ExitingController (Variables|Default|GetDirectorPlayer))
    (if (Variables|Default|GetIsSurvivor)
      (Variables|Default|SetDirectorPlayer (Variables|Default|GetSurvivorPlayer))
      (Variables|Default|SetIsSurvivor false)
      (else
        (Variables|Default|SetIsDirector false)))
    (else
      (Variables|Default|SetIsSurvivor false))))

(event EventHandleStartingNewPlayer
  (params (NewPlayer :type Player%20Controller%20Object%20Reference))
  ;[0.01938 0.01938 0.01938] Add Connecting Player to Queue
  (Utilities|Array|AddUnique (Variables|Default|GetPlayerQueue) NewPlayer)
  (if (== (Utilities|Array|Length (Variables|Default|GetPlayerQueue)) 2)
    (CallFunction|AssignPlayerstoRoles)))

(fn ConstructionScript)